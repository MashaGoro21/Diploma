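; Player component that resets the voxel world and returns the first-person character to the PlayerStart behind an eye-blink transition.
; BeginPlay caches the VoxelWorld and PlayerStart, then binds to the character's blink-close-finished event.
; StartReset, also wired to the C key, waits briefly before closing the blink.
; Once closed, it destroys and recreates the world with global pool creation disabled, teleports the owner and reopens the blink.
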(event `self.ReceiveBeginPlay`
  (bind _returnvalue (`GameplayStatics.GetActorOfClass` "/Script/Voxel.VoxelWorld"))
  (set `self.Voxel World` _returnvalue)
  (bind _returnvalue_2 (`GameplayStatics.GetActorOfClass` "/Script/Engine.PlayerStart"))
  (set `self.Player Start` _returnvalue_2)
  (bind _asbp_first_person_character (cast `/Game/FirstPerson/Blueprints/BP_FirstPersonCharacter` (`self.GetOwner`)))
  (set `self.Player` _asbp_first_person_character)
  (add `/Game/FirstPerson/Blueprints/BP_FirstPersonCharacter.ED_BlinkCloseFinished` _asbp_first_person_character (delegate `OnBlinkFinished`)))

(event `OnBlinkFinished`
  (`self.ResetWorld`))

(event `Key|C`
  (params (Key :type "Key Structure"))
  (:`Pressed`
    (`self.StartReset`)))

(event `StartReset`
  (`KismetSystemLibrary.Delay` 5.0)
  (`/Game/FirstPerson/Blueprints/BP_FirstPersonCharacter.BlinkClose` (`self.Player`)))

(fn `ResetPositon`
  (`Actor.K2_SetActorLocation` (`self.GetOwner`) (`Actor.K2_GetActorLocation` (`self.Player Start`)) false true)
  (`/Game/FirstPerson/Blueprints/BP_FirstPersonCharacter.BlinkOpen` (`self.Player`)))

(fn `ResetWorld`
  (bind _voxel_world (`self.Voxel World`))
  (set `VoxelWorld.bCreateGlobalPool` false _voxel_world)
  (`VoxelWorld.DestroyWorld` _voxel_world)
  (`VoxelWorld.CreateWorld` :`self` _voxel_world)
  (`self.ResetPositon`)
  (return))