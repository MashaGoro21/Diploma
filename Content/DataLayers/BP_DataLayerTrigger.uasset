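; Trigger volume that streams the temple World Partition data layer in and out as the first-person character enters and leaves its box.
; Box overlap begin sets the layer to Activated and prints a debug message, while overlap end sets it to Unloaded.
; BeginPlay also checks existing overlaps, so the layer activates when the character starts inside the box.
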(event `self.ReceiveBeginPlay`
  (if (> (`KismetArrayLibrary.Array_Length` (`PrimitiveComponent.GetOverlappingActors` (`self.Box`) "/Game/FirstPerson/Blueprints/BP_FirstPersonCharacter.BP_FirstPersonCharacter_C")) 0)
    (bind _returnvalue (`WorldPartitionBlueprintLibrary.GetDataLayerManager` :!label _label))
    (`DataLayerManager.SetDataLayerRuntimeState` _returnvalue "/Game/DataLayers/TempleDataLayer.TempleDataLayer" "Activated" false)))

(event `self.Box.OnComponentBeginOverlap`
  (params (OverlappedComponent :type "PrimitiveComponent Object Reference") (OtherActor :type "Actor Object Reference") (OtherComp :type "PrimitiveComponent Object Reference") (OtherBodyIndex :type Integer) (bFromSweep :type Boolean) (SweepResult :type "HitResult Structure (by ref)"))
  (if (`GameplayStatics.ObjectIsA` OtherActor "/Game/FirstPerson/Blueprints/BP_FirstPersonCharacter.BP_FirstPersonCharacter_C")
    (`KismetSystemLibrary.PrintString` "LOADED")
    (goto _label)))

(event `self.Box.OnComponentEndOverlap`
  (params (OverlappedComponent :type "PrimitiveComponent Object Reference") (OtherActor :type "Actor Object Reference") (OtherComp :type "PrimitiveComponent Object Reference") (OtherBodyIndex :type Integer))
  (if (`GameplayStatics.ObjectIsA` OtherActor "/Game/FirstPerson/Blueprints/BP_FirstPersonCharacter.BP_FirstPersonCharacter_C")
    (bind _returnvalue (`WorldPartitionBlueprintLibrary.GetDataLayerManager`))
    (`DataLayerManager.SetDataLayerRuntimeState` _returnvalue "/Game/DataLayers/TempleDataLayer.TempleDataLayer" "Unloaded" false)))

(fn `UserConstructionScript`)