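; BP_Teleport is an environment actor that moves the player to a destination once its linked puzzle is solved.
; On BeginPlay it binds to the PuzzleController's puzzle-solved event, which sets it active and unhides its Plane and that component's children.
; When a player interacts while it is active, it teleports them to the TeleportPoint actor's location without sweeping.
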(event `self.ReceiveBeginPlay`
  (`parent.ReceiveBeginPlay`)
  (add `/Game/Systems/Puzzles/BP_PuzzleController.OnPuzzleSolved` (`self.PuzzleController`) (delegate `Activate`)))

(event `Activate`
  (set `self.Active` true)
  (`SceneComponent.SetHiddenInGame` (`self.Plane`) false true))

(event `/Game/Interfaces/BI_Interactable.Interaction`
  (params (`Player ` :type "/Game/FirstPerson/Blueprints/BP_FirstPersonCharacter Object Reference"))
  (if (`self.Active`)
    (`self.K2_SetActorLocation` `Player ` (`self.K2_GetActorLocation` (`self.TeleportPoint`)) false true)))

(fn `UserConstructionScript`
  (`parent.UserConstructionScript`))