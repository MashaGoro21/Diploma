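; Beer item sample Blueprint that sets up its visual appearance from a Beer data asset.
; InitSample casts the incoming asset to BeerAsset, applies its liquid mesh and material to the LiquidMesh component, then passes it to the parent InitSample.
; A failed cast stops setup before the parent runs.
; The event graph and construction script add no logic of their own.
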(fn `InitSample`
  (params (DataAsset :type "/Game/Objects/DataAssets/Asset Object Reference"))
  (bind _asbeer_asset (cast `/Game/Objects/DataAssets/BeerAsset` DataAsset))
  (`StaticMeshComponent.SetStaticMesh` (`self.LiquidMesh`) (`/Game/Objects/DataAssets/BeerAsset.LiquidMesh` _asbeer_asset))
  (`PrimitiveComponent.SetMaterial` (`self.LiquidMesh`) 0 (`/Game/Objects/DataAssets/BeerAsset.LiquidMaterial` _asbeer_asset))
  (`parent.InitSample` _asbeer_asset))

(fn `UserConstructionScript`
  (`parent.UserConstructionScript`))