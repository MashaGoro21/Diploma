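; Item sample actor that displays a mesh item in the world, configured from a MeshItemAsset data asset.
; InitSample casts the incoming asset to MeshItemAsset, stores it, then applies its main mesh, scale and physics simulation flag to the StaticMesh component.
; Assets of any other type are ignored, and the event graph and construction script add no logic of their own.
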(fn `InitSample`
  (params (DataAsset :type "/Game/Objects/DataAssets/Asset Object Reference"))
  (bind _asmesh_item_asset (cast `/Game/Objects/DataAssets/MeshItemAsset` DataAsset))
  (bind _output_get (set `self.Data Asset` _asmesh_item_asset))
  (`StaticMeshComponent.SetStaticMesh` (`self.StaticMesh`) (`/Game/Objects/DataAssets/MeshItemAsset.MainMesh` _output_get))
  (`SceneComponent.SetRelativeScale3D` (`self.StaticMesh`) (`/Game/Objects/DataAssets/MeshItemAsset.Scale` _output_get))
  (`PrimitiveComponent.SetSimulatePhysics` (`self.StaticMesh`) (`/Game/Objects/DataAssets/MeshItemAsset.EnablePhysics` (`self.Data Asset`))))

(fn `UserConstructionScript`
  (`parent.UserConstructionScript`))