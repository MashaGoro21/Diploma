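; BP_PickaxeSample is a pickaxe item sample actor that configures itself from a data asset.
; Its InitSample runs the parent version, casts the data asset to PickaxeAsset and copies the pickaxe tier.
; If the asset has a valid material instance, it applies it to the first slot of the skeletal mesh.
; The event graph and construction script add no logic of their own.
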(fn `InitSample`
  (params (DataAsset :type "/Game/Objects/DataAssets/Asset Object Reference"))
  (`parent.InitSample` DataAsset)
  (bind _aspickaxe_asset (cast `/Game/Objects/DataAssets/PickaxeAsset` DataAsset))
  (set `self.PickaxeTier` (`/Game/Objects/DataAssets/PickaxeAsset.PickaxeTier` _aspickaxe_asset))
  (bind _materialinst (`/Game/Objects/DataAssets/PickaxeAsset.MaterialInst` _aspickaxe_asset))
  (`/Engine/EditorBlueprintResources/StandardMacros.IsValid` _materialinst
    (:`Is Valid`
      (`PrimitiveComponent.SetMaterial` (`self.SkeletalMesh`) 0 _materialinst))))

(fn `UserConstructionScript`
  (`parent.UserConstructionScript`))