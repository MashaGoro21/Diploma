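; BP_ConsumableObjectMaster is a base Blueprint for consumable item objects, with no item behavior of its own.
; Consume is a stub that always returns false, leaving the actual effect to be defined elsewhere.
; ReturnPlayerCharacter lazily caches player 0's character as BP_FirstPersonCharacter and returns it.
; The event graph holds only disabled default events, and the construction script just calls its parent.
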(fn `Consume`
  (returns (Success :type Boolean))
  (return false))

(fn `ReturnPlayerCharacter`
  (returns (PlayerCharacter :type "/Game/FirstPerson/Blueprints/BP_FirstPersonCharacter Object Reference"))
  (bind _playercharacter (`self.PlayerCharacter`))
  (`/Engine/EditorBlueprintResources/StandardMacros.IsValid` _playercharacter
    (:`Is Valid`
      _)
    (:`Is Not Valid`
      (bind _asbp_first_person_character (cast `/Game/FirstPerson/Blueprints/BP_FirstPersonCharacter` (`GameplayStatics.GetPlayerCharacter` 0)))
      (set `self.PlayerCharacter` _asbp_first_person_character)))
  (return _playercharacter))

(fn `UserConstructionScript`
  (`parent.UserConstructionScript`))