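; Base Blueprint for item objects that a player can highlight and pick up.
; Interaction passes the player to ItemDataComponent's PickUpItem, and HighlightObject defers to the parent implementation, both only while IsActive is true.
; ChangeState sets that flag from its IsItem input, and ChangeItemQuantity writes the quantity into ItemDataComponent.
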(event `/Game/Interfaces/BI_Interactable.Interaction`
  (params (`Player ` :type "/Game/FirstPerson/Blueprints/BP_FirstPersonCharacter Object Reference"))
  (if (`self.IsActive`)
    (`/Game/Systems/Items/Components/ItemDataComponent.Pick Up Item` (`self.ItemDataComponent`) `Player `)))

(event `/Game/Interfaces/BI_Interactable.HighlightObject`
  (params (IsSelected :type Boolean))
  (if (`self.IsActive`)
    (`parent.HighlightObject` IsSelected)))

(event `/Game/Interfaces/BI_Item.ChangeState`
  (params (IsItem :type Boolean))
  (set `self.IsActive` IsItem))

(fn `Change Item Quantity`
  (params (Quantity :type Integer))
  (set `/Game/Systems/Items/Components/ItemDataComponent.Quantity` Quantity (`self.ItemDataComponent`)))

(fn `UserConstructionScript`
  (`parent.UserConstructionScript`))