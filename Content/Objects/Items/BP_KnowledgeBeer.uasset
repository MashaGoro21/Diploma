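; BP_KnowledgeBeer is a consumable item that increases the consuming player's knowledge.
; Its Consume override runs the parent logic, then calls IncreaseKnowledge on the player.
; It then looks up the KnowledgeIncrease row in the TutorialData table and shows its icon and message in a WB_TutorialPopUp widget added to the viewport.
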(fn `Consume`
  (params (`Consuming Player` :type "/Game/FirstPerson/Blueprints/BP_FirstPersonCharacter Object Reference"))
  (returns (Success :type Boolean))
  (bind _success (`parent.Consume` `Consuming Player`))
  (`/Game/FirstPerson/Blueprints/BP_FirstPersonCharacter.Increase Knowledge` `Consuming Player`)
  (bind _returnvalue (`|GetDataTableRow` "/Game/Systems/Tutorial/TutorialData/TutorialData.TutorialData" "KnowledgeIncrease")
    (:`then`
      (bind (_tutorialid _title _message _icon) (break `/Game/Systems/Tutorial/TutorialData/FTutorialStruct` _returnvalue))
      (bind _returnvalue_2 (`|CreateWidget` "/Game/Systems/Tutorial/Widgets/WB_TutorialPopUp.WB_TutorialPopUp_C" null _icon _message))
      (`UserWidget.AddToViewport` _returnvalue_2 0)
      (return _success))))

(fn `UserConstructionScript`
  (`parent.UserConstructionScript`))