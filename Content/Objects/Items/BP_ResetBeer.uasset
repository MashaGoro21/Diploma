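; BP_ResetBeer is a consumable beer item that starts a reset on the player who drinks it.
; Its Consume override runs the parent logic, calls StartReset on the consuming player's BPCResetComponent, then returns the parent's result.
; The reset behavior lives in that component, and the event graph holds only disabled default events.
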(fn `Consume`
  (params (`Consuming Player` :type "/Game/FirstPerson/Blueprints/BP_FirstPersonCharacter Object Reference"))
  (returns (Success :type Boolean))
  (bind _success (`parent.Consume` `Consuming Player`))
  (`/Game/BPC_ResetComponent.StartReset` (`/Game/FirstPerson/Blueprints/BP_FirstPersonCharacter.BPC_ResetComponent` `Consuming Player`))
  (return _success))

(fn `UserConstructionScript`
  (`parent.UserConstructionScript`))