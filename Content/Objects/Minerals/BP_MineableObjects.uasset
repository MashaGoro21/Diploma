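; Base Blueprint for a mineable object that loses one Durability per Mine call and breaks on the final hit.
; Breaking calls ExplodeObject, which spawns a DroppingItem along SpawnSpline points (indexed from 1, not 0), prints a debug string, then destroys the actor.
; Explode's delayed destroy follows that immediate destroy, and a geometry-collection radial impulse is left unconnected.
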(event `self.ReceiveBeginPlay`
  (`parent.ReceiveBeginPlay`))

(event `Explode`
  (`self.ExplodeObject`)
  (`KismetSystemLibrary.Delay` (`self.Dissapear`))
  (`self.K2_DestroyActor`))

(fn `ExplodeObject`
  (bind _spawnspline (`self.SpawnSpline`))
  (for _index (range 1 (+ (`SplineComponent.GetNumberOfSplinePoints` _spawnspline) 1))
    (`|SpawnActorFromClass` (`self.DroppingItem`) (`KismetMathLibrary.Conv_VectorToTransform` (`SplineComponent.GetLocationAtSplinePoint` _spawnspline _index "World")) "Undefined" "MultiplyWithRoot" null null)
    (`KismetSystemLibrary.PrintString` "Hello"))
  (`self.K2_DestroyActor`))

(fn `Mine`
  (bind _durability (`self.Durability`))
  (if (> _durability 1)
    (`/Engine/EditorBlueprintResources/StandardMacros.DecrementInt` (`self.Durability`) :!label _label)
    (elif (> _durability 0)
      (`self.Explode`)
      (goto _label))))

(fn `UserConstructionScript`
  (`parent.UserConstructionScript`))