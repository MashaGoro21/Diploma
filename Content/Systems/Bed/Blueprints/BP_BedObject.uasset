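; BP_BedObject is an interactable bed that puts the player to sleep and saves the game.
; Interaction disables input, hides the right hand and light sphere after a delay, and plays a sleeping sound.
; Two timelines drive MPC_Blink parameters to close and reopen the eyes, requesting a BP_GameInstance save between them.
; Waking restores input and hand visuals and calls the player's location reset; the WB_Sleeping animation chain is unconnected.
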(event `/Game/Interfaces/BI_Interactable.Interaction`
  (params (`Player ` :type "/Game/FirstPerson/Blueprints/BP_FirstPersonCharacter Object Reference"))
  (bind _returnvalue (`GameplayStatics.GetPlayerController` 0))
  (bind _player (`self.Player`))
  (bind _player_2 (`self.Player`))
  (bind _lightsphere (`/Game/FirstPerson/Blueprints/BP_FirstPersonCharacter.LightSphere` _player_2))
  (bind _output_get (set `self.Player` `Player `))
  (set `/Game/FirstPerson/Blueprints/BP_FirstPersonCharacter.IsSleeping` true _output_get)
  (`self.DisableInput` _output_get _returnvalue)
  (`KismetSystemLibrary.Delay` (`/Game/FirstPerson/Blueprints/BP_FirstPersonCharacter.WaitingForPuttingDownTime` _output_get))
  (`SceneComponent.SetHiddenInGame` (`/Game/FirstPerson/Blueprints/BP_FirstPersonCharacter.RightHand` _output_get) true false)
  (`SceneComponent.SetHiddenInGame` (`/Game/FirstPerson/Blueprints/BP_FirstPersonCharacter.LightSphere` _output_get) true false)
  (`AudioComponent.Play` (`/Game/FirstPerson/Blueprints/BP_FirstPersonCharacter.SleepingSound` (`self.Player`)) 0.0)
  (`KismetSystemLibrary.Delay` (`/Game/FirstPerson/Blueprints/BP_FirstPersonCharacter.PrepareForSleepTime` _output_get))
  (bind (_direction _newtrack_0) (`Timeline|TL_BlinkClose` :!via `PlayFromStart`)
    (:`Update`
      (`KismetMaterialLibrary.SetScalarParameterValue` "/Game/Material/Blinking/MPC_Blink.MPC_Blink" "EyeHardness" _newtrack_0)
      (`KismetMaterialLibrary.SetScalarParameterValue` "/Game/Material/Blinking/MPC_Blink.MPC_Blink" "AmountOpened" _newtrack_0))
    (:`Finished`
      (`self.Saving`)
      (bind (_direction_2 _newtrack_0_2) (`Timeline|TL_BlinkOpen` :!via `PlayFromStart`)
        (:`Update`
          (`KismetMaterialLibrary.SetScalarParameterValue` "/Game/Material/Blinking/MPC_Blink.MPC_Blink" "EyeHardness" _newtrack_0_2)
          (`KismetMaterialLibrary.SetScalarParameterValue` "/Game/Material/Blinking/MPC_Blink.MPC_Blink" "AmountOpened" _newtrack_0_2))
        (:`Finished`
          (`Widget.RemoveFromParent` (`WidgetComponent.GetWidget` (`self.Widget_0`)))
          (`self.EnableInput` _player _returnvalue)
          (set `/Game/FirstPerson/Blueprints/BP_FirstPersonCharacter.IsSleeping` false _player)
          (`SceneComponent.SetHiddenInGame` (`/Game/FirstPerson/Blueprints/BP_FirstPersonCharacter.RightHand` _player_2) false false)
          (`/Game/FirstPerson/Blueprints/BP_FirstPersonCharacter.ED_ResetLocation` (`self.Player`))
          (if (`/Game/FirstPerson/Blueprints/BP_FirstPersonCharacter.LeftHandActive?` _player_2)
            (`SceneComponent.SetHiddenInGame` _lightsphere false false)
            (else
              (`SceneComponent.SetHiddenInGame` _lightsphere true false))))))))

(event `Saving`
  (bind _asbp_game_instance (cast `/Game/Systems/Save/BP_GameInstance` (`GameplayStatics.GetGameInstance`)))
  (`/Game/Systems/Save/BP_GameInstance.RequestSave` _asbp_game_instance false))

(fn `UserConstructionScript`
  (`parent.UserConstructionScript`))