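; Brewing station that turns a mug, mineral and plant from its three-slot inventory into a product, likely beer.
; Slot changes update item actors, animate the fuel and plant compartments with timelines, and update the brew button according to whether all slots are filled.
; Brewing matches plant and mineral against DT_BrewingRecipe, plays a timed pour with product-specific liquid material, then replaces the ingredients and mug with the product.
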(event `self.ReceiveBeginPlay`
  (`parent.ReceiveBeginPlay`)
  (bind _aswb_brewing_station (cast `/Game/Systems/Brewing/Widgets/WB_BrewingStation` (`self.MainWidget`)))
  (set `self.Brewing Widget` _aswb_brewing_station)
  (add `/Game/Systems/Brewing/Widgets/WB_BrewingStation.ED_MakeBear` (`self.Brewing Widget`) (`|CreateDelegate` :!event `StartBrewingEvent`)))

(event `PlantCompartmentEvent`
  ; OpenClose Animation
  (bind _output_get (set `self.PlantOpen` (not (`self.PlantOpen`))))
  (if _output_get
    (bind (_direction `_новая_дорожка_0`) (`Timeline|Шкала времени_1` :!via `Reverse` :!label _label)
      (:`Update`
        (`SceneComponent.K2_SetRelativeRotation` (`self.Scene_0`) (`KismetMathLibrary.MakeRotator` (`KismetMathLibrary.Lerp` 158.0 0.0 `_новая_дорожка_0`)) false false)))
    (else
      (goto _label))))

(event `FuelCompartmentEvent`
  ; OpenClose Animation
  (bind _output_get (set `self.FuelOpen` (not (`self.FuelOpen`))))
  (if _output_get
    (bind (_direction `_новая_дорожка_0`) (`Timeline|Шкала времени_0` :!via `Reverse` :!label _label_2)
      (:`Update`
        (`SceneComponent.K2_SetRelativeRotation` (`self.Scene1`) (`KismetMathLibrary.MakeRotator` 180.0 (`KismetMathLibrary.Lerp` -30.0 180.0 `_новая_дорожка_0`) 180.0) false false)))
    (else
      (goto _label_2))))

(event `self.StartInspection`
  (`parent.StartInspection`))

(event `OnInventoryUpdated`
  (params (SlotId :type Integer))
  (bind ((`IsEmpty_10_FE7A134C4724E51CB84AA3B236CF5534` _isempty) (`Item_26_E76130004EA97320794B31AFED0241D9` _item)) (break `/Game/Systems/Inventory/Slots/Structs/FSlotStruct` (`|GetArrayItem` (`/Game/Systems/Inventory/Components/BPC_MasterInventorySystem.Content` (`self.StationInventory`)) SlotId)))
  (`/Game/Systems/Brewing/Widgets/WB_BrewingStation.UptadeInventory` (`self.Brewing Widget`))
  (switch `int` SlotId
    (:`0`
      (`self.SetItem` _item (`self.MugActor`))
      (`AudioComponent.Play` (`self.MugDroppingSound`) 0.0)
      (`self.BrewingInitialize` :!label _label_3))
    (:`1`
      (if (xor _isempty (`self.FuelOpen`))
        (`self.SetItem` _item (`self.MineralActor`))
        (`self.FuelCompartmentEvent`)
        (`AudioComponent.Play` (`self.MineralDroppingSound`) 0.0)
        (goto _label_3)))
    (:`2`
      (if (xor _isempty (`self.PlantOpen`))
        (`self.SetItem` _item (`self.PlantActor`))
        (`self.PlantCompartmentEvent`)
        (`AudioComponent.Play` (`self.PlantDroppingSound`) 0.0)
        (goto _label_3)))))

(event `StartBrewingEvent`
  (bind (_isfound _product) (`self.CheckIngredients`))
  (if _isfound
    (bind (_value _returnvalue) (`BlueprintMapLibrary.Map_Find` (`self.LiquidsMap`) _product))
    (if _returnvalue
      (`PrimitiveComponent.SetMaterial` (`self.BeerSteam`) 0 _value))
    (`AudioComponent.Play` (`self.PouringBeerSound`) 0.0)
    (`Widget.SetVisibility` (`self.MainWidget`) "Collapsed")
    (`SceneComponent.SetHiddenInGame` (`self.BeerSteam`) false false)
    (`KismetSystemLibrary.Delay` 2.0)
    (`Widget.SetVisibility` (`self.MainWidget`) "Visible")
    (`SceneComponent.SetHiddenInGame` (`self.BeerSteam`) true false)
    (bind _returnvalue_2 (`|GetDataTableRow` "/Game/Systems/Brewing/DT_BrewingRecipe.DT_BrewingRecipe" _product)
      (:`then`
        (`/Game/Systems/Inventory/Components/BPC_MasterInventorySystem.Remove From Slot` (`self.StationInventory`) (`self.PlantNumber`))
        (`/Game/Systems/Inventory/Components/BPC_MasterInventorySystem.Remove From Slot` (`self.StationInventory`) (`self.MineralNumber`))
        (`/Game/Systems/Inventory/Components/BPC_MasterInventorySystem.Remove From Slot` (`self.StationInventory`) 0)
        (`/Game/Systems/Inventory/Components/BPC_MasterInventorySystem.Add To Slot` (`self.StationInventory`) 0 (`.Product_13_F86D88B04A1D148E14C0A2B191E3730F` (break `/Game/Systems/Brewing/FBrewingStruct` _returnvalue_2)))
        (`/Game/Systems/Brewing/Widgets/WB_BrewingStation.UptadeInventory` (`self.Brewing Widget`))))))

(fn `BrewingInitialize`
  (`/Game/Systems/Brewing/Widgets/WB_BrewingStation.ButtonInitialize` (`self.Brewing Widget`) (and (not (`self.CheckSlotStatus` 2)) (not (`self.CheckSlotStatus` 1)) (not (`self.CheckSlotStatus` 0)))))

(fn `CheckIngredients`
  (returns (IsFound :type Boolean) (Product :type Name))
  (bind _outrownames (`DataTableFunctionLibrary.GetDataTableRowNames` "/Game/Systems/Brewing/DT_BrewingRecipe.DT_BrewingRecipe"))
  (for _array_element _outrownames
    (bind _returnvalue (`|GetDataTableRow` "/Game/Systems/Brewing/DT_BrewingRecipe.DT_BrewingRecipe" _array_element)
      (:`then`
        (bind (_plant _mineral _product) (break `/Game/Systems/Brewing/FBrewingStruct` _returnvalue))
        (bind _returnvalue_2 (and (`self.CompareItems` _plant (`.Item_26_E76130004EA97320794B31AFED0241D9` (break `/Game/Systems/Inventory/Slots/Structs/FSlotStruct` (`|GetArrayItem` (`/Game/Systems/Inventory/Components/BPC_MasterInventorySystem.Content` (`self.StationInventory`)) (`self.PlantNumber`))))) (`self.CompareItems` _mineral (`.Item_26_E76130004EA97320794B31AFED0241D9` (break `/Game/Systems/Inventory/Slots/Structs/FSlotStruct` (`|GetArrayItem` (`/Game/Systems/Inventory/Components/BPC_MasterInventorySystem.Content` (`self.StationInventory`)) (`self.MineralNumber`)))))))
        (if _returnvalue_2
          (return _returnvalue_2 _product)))))
  (return false "None"))

(fn `CheckSlotStatus`
  (params (SlotNumber :type Integer))
  (returns (IsEmpty :type Boolean))
  (return (`.IsEmpty_10_FE7A134C4724E51CB84AA3B236CF5534` (break `/Game/Systems/Inventory/Slots/Structs/FSlotStruct` (`|GetArrayItem` (`/Game/Systems/Inventory/Components/BPC_MasterInventorySystem.Content` (`self.StationInventory`)) SlotNumber)))))

(fn `CompareItems`
  (params (Item1 :type Name) (Item2 :type Name))
  (returns (SameItem :type Boolean))
  (return (== Item1 Item2)))

(fn `SetMeshes`
  (set `self.Meshes` (`|MakeArray` (`self.MainMesh`) (`self.StaticMesh2`) (`self.StaticMesh1`) :!type "MeshComponent Object Reference")))

(fn `UserConstructionScript`)