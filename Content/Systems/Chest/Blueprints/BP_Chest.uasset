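; BP_Chest is an inspectable chest that swings open when inspection starts and closes when it ends.
; StartInspection plays the open sound, binds to the OnClose dispatcher, calls the parent's inspection logic and plays a Timeline that lerps Scene0's pitch.
; On close, it plays the close sound, unbinds the event and reverses the same Timeline.
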(event `self.StartInspection`
  (`AudioComponent.Play` (`self.ChestOpenSound`) 0.0)
  (add `self.OnClose` (delegate `OnClose_Event`))
  (`parent.StartInspection`)
  (bind (_direction `_новая_дорожка_0`) (`Timeline|Timeline` :!label _label)
    (:`Update`
      (`SceneComponent.K2_SetRelativeRotation` (`self.Scene_0`) (`KismetMathLibrary.MakeRotator` 0.0 (`KismetMathLibrary.Lerp` -1.0 100.0 `_новая_дорожка_0`)) false false))))

(event `OnClose_Event`
  (`AudioComponent.Play` (`self.ChestCloseSound`) 0.0)
  (remove `self.OnClose` (delegate `OnClose_Event`))
  (goto _label :!via `Reverse`))

(fn `UserConstructionScript`
  (`parent.UserConstructionScript`))