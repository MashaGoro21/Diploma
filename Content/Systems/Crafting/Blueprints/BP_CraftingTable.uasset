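; Crafting table actor that lets the player craft items from recipes through a crafting widget.
; On BeginPlay it binds widget and open events, refreshing the recipe list from the player when opened.
; Crafting converts recipe materials into an ID-to-quantity map for the player's item check, reports the result, and on success adds the product to the inventory.
; Widget entries regenerate after each attempt, and player input is re-enabled when the widget animation finishes.
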(event `self.ReceiveBeginPlay`
  (`parent.ReceiveBeginPlay`)
  (bind _asw_crafting_widget (cast `/Game/Systems/Crafting/Widgets/W_Crafting_Widget` (`self.MainWidget`)))
  (bind _asdwarf_hud (cast `/Game/Widgets/HUD/DwarfHUD` (`PlayerController.GetHUD` (`GameplayStatics.GetPlayerController` 0))))
  (set `self.DwarfHUD` (`|ConvertAsset` _asdwarf_hud))
  (set `self.CraftingWidget` _asw_crafting_widget)
  (add `/Game/Systems/Crafting/Widgets/W_Crafting_Widget.CraftED` (`self.CraftingWidget`) (delegate `Craft`))
  (add `self.OnOpen` (delegate `Started Crafting`))
  (add `/Game/Systems/Crafting/Widgets/W_Crafting_Widget.OnAnimationFinishedED` (`self.CraftingWidget`) (delegate `Finished Crafting`)))

(event `Craft`
  (params (Recipe :type "/Game/Systems/Crafting/Data/RecipeStruct Structure"))
  (`self.Scan Inventory` (`self.Player`) Recipe)
  (`/Game/Systems/Crafting/Widgets/W_Crafting_Widget.Regenerate Entries` (`self.CraftingWidget`)))

(event `Started Crafting`
  (`/Game/Systems/Crafting/Widgets/W_Crafting_Widget.Update recipes` (`self.CraftingWidget`) (`self.Player`)))

(event `Finished Crafting`
  (`self.EnableInput` (`self.Player`) (`self.Player Controller`)))

(fn `ConvertToMap`
  (params (Array :type "Array of /Game/Systems/Items/Data/Struct/FItemStruct Structure"))
  (returns (Map :type "Map of Name to Integer"))
  (locals (LocalMap :type "Map of Name to Integer"))
  (bind _localmap (`local.LocalMap`))
  (for _array_element Array
    (bind (_itemid _quantity) (break `/Game/Systems/Items/Data/Struct/FItemStruct` _array_element))
    (`BlueprintMapLibrary.Map_Add` _localmap _itemid _quantity))
  (return _localmap))

(fn `Scan Inventory`
  (params (`Player inventory` :type "/Game/FirstPerson/Blueprints/BP_FirstPersonCharacter Object Reference") (Recipe :type "/Game/Systems/Crafting/Data/RecipeStruct Structure"))
  (bind (_materials _product) (break `/Game/Systems/Crafting/Data/RecipeStruct` Recipe))
  (bind _map (`self.ConvertToMap` _materials))
  (bind _enough_ (`/Game/FirstPerson/Blueprints/BP_FirstPersonCharacter.CheckItems` `Player inventory` _map))
  (`/Game/Systems/Crafting/Widgets/W_Crafting_Widget.Crafting Result` (`self.CraftingWidget`) _enough_)
  (if _enough_
    (`/Game/Systems/Inventory/Components/BPC_PlayerInventory.PickUpItem` (`/Game/FirstPerson/Blueprints/BP_FirstPersonCharacter.BPC_PlayerInventory` `Player inventory`) (`.ItemId_2_D15E650D447F179120E90DBF367FFFF8` (break `/Game/Systems/Items/Data/Struct/FItemStruct` _product)))))

(fn `SetWidget`
  (params (Widget :type "UserWidget Class Reference"))
  (bind _returnvalue (`|CreateWidget` Widget (`GameplayStatics.GetPlayerController` 0)))
  (set `self.MainWidget` _returnvalue))

(fn `UserConstructionScript`
  (`parent.UserConstructionScript`))