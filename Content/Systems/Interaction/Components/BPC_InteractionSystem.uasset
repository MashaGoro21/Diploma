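; Interaction component that finds, highlights and triggers interactable actors for the player.
; TraceEvent takes start and end points, runs a multi-sphere trace and picks the first hit implementing BI_Interactable.
; Highlight messages fire only when the target changes, switching off the old actor and on the new one.
; IA_Interact sets a pressed flag that TraceEvent consumes, sending InteractionMessage to the target and clearing its highlight.
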(event `self.TraceEvent`
  (params (Start :type "Vector Structure") (End :type "Vector Structure"))
  ; Interact
  (bind _outhits (`KismetSystemLibrary.SphereTraceMulti` Start End (`self.Radius`) "TraceTypeQuery3"))
  (`self.InitializeActorObject` _outhits)
  (`self.HighlightInteractableObject`)
  (if (and (`self.IsInteractionWasPressed`) (`self.IsImplement`))
    (message `/Game/Interfaces/BI_Interactable.Interaction` (`self.CurrentActorRef`) (`self.Player`))
    (set `self.New Actor` null)
    (`self.HighlightInteractableObject`)
    (set `self.IsInteractionWasPressed` false)))

(event `EnhancedInput|/Game/FirstPerson/Input/Actions/IA_Interact`
  (params (ActionValue :type Boolean) (ElapsedSeconds :type "Float (double-precision)") (TriggeredSeconds :type "Float (double-precision)") (InputAction :type "InputAction Object Reference" :default "/Game/FirstPerson/Input/Actions/IA_Interact.IA_Interact"))
  ; Interact
  (:`Triggered`
    (set `self.IsInteractionWasPressed` ActionValue :!label _label))
  (:`Canceled`
    (goto _label))
  (:`Completed`
    (goto _label)))

(fn `HighlightInteractableObject`
  (if (!= (`self.New Actor`) (`self.CurrentActorRef`))
    (set `self.IsImplement` (`KismetSystemLibrary.DoesImplementInterface` (`self.New Actor`) "/Game/Interfaces/BI_Interactable.BI_Interactable_C"))
    (`/Engine/EditorBlueprintResources/StandardMacros.IsValid` (`self.CurrentActorRef`)
      (:`Is Valid`
        (message `/Game/Interfaces/BI_Interactable.HighlightObject` (`self.CurrentActorRef`) false))
      (:`Is Not Valid`
        _))
    (if (`self.IsImplement`)
      (bind _output_get (set `self.CurrentActorRef` (`self.New Actor`)))
      (message `/Game/Interfaces/BI_Interactable.HighlightObject` _output_get true)
      (else
        (set `self.CurrentActorRef` null)))))

(fn `InitializeActorObject`
  (params (`Out Hits` :type "Array of HitResult Structure"))
  (if (> (`KismetArrayLibrary.Array_Length` `Out Hits`) 0)
    (for _array_element `Out Hits`
      (bind (_bblockinghit _binitialoverlap _time _distance _location _impactpoint _normal _impactnormal _physmat _hitactor) (`GameplayStatics.BreakHitResult` _array_element))
      (bind _output_get (set `self.IsImplement` (`KismetSystemLibrary.DoesImplementInterface` _hitactor "/Game/Interfaces/BI_Interactable.BI_Interactable_C")))
      (if _output_get
        (set `self.New Actor` _hitactor)
        (break)
        (else
          (set `self.New Actor` null))))
    (else
      (set `self.New Actor` null))))