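; Equipment inventory component for BP_FirstPersonCharacter that manages the selected slot and shows its item in the player's right hand.
; Enhanced Input actions select one of four slots directly or cycle with wraparound once accumulated scroll input crosses a threshold.
; Slot changes and updates to the selected slot look up the ItemData table to set the hand item.
; A use action consumes the parent's UseItem, and dispatchers broadcast selection and equipment changes.
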(event `self.ReceiveBeginPlay`
  (`parent.ReceiveBeginPlay`)
  (bind _asbp_first_person_character (cast `/Game/FirstPerson/Blueprints/BP_FirstPersonCharacter` (`self.GetOwner`)))
  (set `self.Player` _asbp_first_person_character)
  (add `self.InventoryUpdated` (delegate `OnInventoryUpdated`))
  (`self.OnInventoryUpdated` 0))

(event `OnInventoryUpdated` :!signature `self.InventoryUpdated`
  (params (SlotId :type Integer))
  (`self.OnEquipmentUpdated`)
  (if (== SlotId (`self.SelectedSlot`))
    (`self.SetSelectedItem` (`self.SelectedSlot`))))

(event `ChangeSelectedSlot`
  (params (SlotId :type Integer))
  (if (`self.IsValidToChange` SlotId)
    (bind _output_get (set `self.SelectedSlot` SlotId))
    (`self.SetSelectedItem` _output_get)))

(event `EnhancedInput|/Game/FirstPerson/Input/Actions/IA_FirstSlot`
  (params (ActionValue :type Boolean) (ElapsedSeconds :type "Float (double-precision)") (TriggeredSeconds :type "Float (double-precision)") (InputAction :type "InputAction Object Reference" :default "/Game/FirstPerson/Input/Actions/IA_FirstSlot.IA_FirstSlot"))
  (:`Triggered`
    (`self.ChangeSelectedSlot` 0)))

(event `EnhancedInput|/Game/FirstPerson/Input/Actions/IA_SecondSlot`
  (params (ActionValue :type Boolean) (ElapsedSeconds :type "Float (double-precision)") (TriggeredSeconds :type "Float (double-precision)") (InputAction :type "InputAction Object Reference" :default "/Game/FirstPerson/Input/Actions/IA_SecondSlot.IA_SecondSlot"))
  (:`Triggered`
    (`self.ChangeSelectedSlot` 1)))

(event `EnhancedInput|/Game/FirstPerson/Input/Actions/IA_ThirdSlot`
  (params (ActionValue :type Boolean) (ElapsedSeconds :type "Float (double-precision)") (TriggeredSeconds :type "Float (double-precision)") (InputAction :type "InputAction Object Reference" :default "/Game/FirstPerson/Input/Actions/IA_ThirdSlot.IA_ThirdSlot"))
  (:`Triggered`
    (`self.ChangeSelectedSlot` 2)))

(event `EnhancedInput|/Game/FirstPerson/Input/Actions/IA_FourthSlot`
  (params (ActionValue :type Boolean) (ElapsedSeconds :type "Float (double-precision)") (TriggeredSeconds :type "Float (double-precision)") (InputAction :type "InputAction Object Reference" :default "/Game/FirstPerson/Input/Actions/IA_FourthSlot.IA_FourthSlot"))
  (:`Triggered`
    (`self.ChangeSelectedSlot` 3)))

(event `EnhancedInput|/Game/FirstPerson/Input/Actions/IA_ScrollSlot`
  (params (ActionValue :type "Float (double-precision)") (ElapsedSeconds :type "Float (double-precision)") (TriggeredSeconds :type "Float (double-precision)") (InputAction :type "InputAction Object Reference" :default "/Game/FirstPerson/Input/Actions/IA_ScrollSlot.IA_ScrollSlot"))
  (:`Triggered`
    (bind _output_get (set `self.ScrollAccumulatedValue` (+ ActionValue (`self.ScrollAccumulatedValue`))))
    (if (>= _output_get (`self.ScrollThreshold`))
      (set `self.ScrollAccumulatedValue` 0.0)
      (`self.PrevSlot`)
      (else
        (bind _result (`/Engine/EditorBlueprintResources/StandardMacros.NegateFloat` (`|Copy` (`self.ScrollThreshold`)))
          (:`  `
            (if (<= (`self.ScrollAccumulatedValue`) _result)
              (set `self.ScrollAccumulatedValue` 0.0)
              (`self.NextSlot`))))))))

(event `EnhancedInput|/Game/FirstPerson/Input/Actions/IA_UseItem`
  (params (ActionValue :type Boolean) (ElapsedSeconds :type "Float (double-precision)") (TriggeredSeconds :type "Float (double-precision)") (InputAction :type "InputAction Object Reference" :default "/Game/FirstPerson/Input/Actions/IA_UseItem.IA_UseItem"))
  (:`Triggered`
    (`self.UseItem` (`self.SelectedSlot`))
    (`self.OnEquipmentUpdated`)))

(fn `IsValidToChange`
  (params (SlotId :type Integer))
  (returns (ReturnValue :type Boolean))
  (return (and (!= SlotId (`self.SelectedSlot`)) (< SlotId (`self.Inventory Size`)))))

(fn `NextSlot`
  (locals (LocalSelectedSlot :type Integer))
  (bind _output_get (set `local.LocalSelectedSlot` (+ (`self.SelectedSlot`) 1)))
  (if (>= _output_get (`self.Inventory Size`))
    (set `local.LocalSelectedSlot` 0))
  (`self.ChangeSelectedSlot` (`local.LocalSelectedSlot`))
  (`KismetSystemLibrary.PrintString` "NextSlot"))

(fn `PrevSlot`
  (locals (LocalSelectedSlot :type Integer))
  (bind _output_get (set `local.LocalSelectedSlot` (- (`self.SelectedSlot`) 1)))
  (if (< _output_get 0)
    (set `local.LocalSelectedSlot` (- (`self.Inventory Size`) 1)))
  (`self.ChangeSelectedSlot` (`local.LocalSelectedSlot`))
  (`KismetSystemLibrary.PrintString` "Prevslot"))

(fn `SetSelectedItem`
  (params (SlotId :type Integer))
  (bind ((`Item_26_E76130004EA97320794B31AFED0241D9` _item)) (break `/Game/Systems/Inventory/Slots/Structs/FSlotStruct` (`|GetArrayItem` (`self.Content`) SlotId)))
  (`self.OnSlotSelected` SlotId)
  (if (>= SlotId 0)
    (bind _returnvalue (`|GetDataTableRow` "/Game/Systems/Items/Data/ItemData.ItemData" _item)
      (:`then`
        (`/Game/FirstPerson/Blueprints/BP_FirstPersonCharacter.SetItemToRightHand` (`self.Player`) (`.ItemAsset_36_1B4865824EB956846D6490BC657ABC3E` (break `/Game/Systems/Items/Data/Struct/FItemDataStruct` _returnvalue))))
      (:`RowNotFound`
        (`/Game/FirstPerson/Blueprints/BP_FirstPersonCharacter.SetItemToRightHand` (`self.Player`) null)))
    (`KismetSystemLibrary.PrintString` (`KismetStringLibrary.Concat_StrStr` (`KismetStringLibrary.Conv_NameToString` _item) "Chuj"))))