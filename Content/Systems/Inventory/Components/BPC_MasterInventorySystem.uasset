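; Slot-based inventory component that stores item IDs, resolves them through a data table, and notifies on slot changes.
; Transfers swap slots within or between inventories, checking only the destination slot's accepted type, or auto-pick an empty compatible slot.
; Using a consumable removes it, spawns its actor and sends it the owning first-person character.
; Contents save and load through the GameInstance's SaveGame map, keyed by component path name.
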(event `self.ReceiveBeginPlay`
  (bind _returnvalue (`GameplayStatics.GetGameInstance`))
  (bind _returnvalue_2 (`KismetSystemLibrary.GetPathName` self))
  (bind _asbp_game_instance (cast `/Game/Systems/Save/BP_GameInstance` _returnvalue))
  (`KismetArrayLibrary.Array_Resize` (`self.Content`) (`self.Inventory Size`))
  (bind _inventorymap (`/Game/Systems/Save/BP_SaveGame.InventoryMap` (`/Game/Systems/Save/BP_GameInstance.SaveGameRef` _asbp_game_instance)))
  (if (not (`BlueprintMapLibrary.Map_Contains` _inventorymap _returnvalue_2))
    (`BlueprintMapLibrary.Map_Add` _inventorymap _returnvalue_2 (make `/Game/Systems/Save/FInventorySave` (`self.Content`))))
  (message `/Game/Systems/Save/BPI_Persistence.RequestLoad` _returnvalue self))

(event `/Game/Systems/Save/BPI_Saveable.SaveData`
  (params (SaveGameRef :type "/Game/Systems/Save/BP_SaveGame Object Reference"))
  (`BlueprintMapLibrary.Map_Add` (`/Game/Systems/Save/BP_SaveGame.InventoryMap` SaveGameRef) (`KismetSystemLibrary.GetPathName` self) (make `/Game/Systems/Save/FInventorySave` (`self.Content`))))

(event `/Game/Systems/Save/BPI_Saveable.LoadData`
  (params (SaveGameRef :type "/Game/Systems/Save/BP_SaveGame Object Reference"))
  (set `self.Content` (`.Content_8_0CA98DDB4BC15C638C7999AFBAF264AE` (break `/Game/Systems/Save/FInventorySave` (`BlueprintMapLibrary.Map_Find` (`/Game/Systems/Save/BP_SaveGame.InventoryMap` SaveGameRef) (`KismetSystemLibrary.GetPathName` self)))))
  (`self.InventoryUpdated` 0))

(fn `Add To Slot`
  (params (`Target slot` :type Integer) (Item :type Name))
  (setmembers `/Game/Systems/Inventory/Slots/Structs/FSlotStruct` :`StructRef` (`|GetArrayItem` (`self.Content`) `Target slot`) :`IsEmpty` (== Item "None") :`Item` Item)
  (`self.InventoryUpdated` (`local.Target slot`)))

(fn `FindSuitableSlot`
  (params (SourceIndex :type Integer) (SourceInventory :type "/Game/Systems/Inventory/Components/BPC_MasterInventorySystem Object Reference"))
  (returns (SlotIndex :type Integer))
  (for _index (range (+ (`self.Inventory Size`) 1))
    (bind _isempty (`self.IsSlotEmpty` _index self))
    (if _isempty
      (bind _valid (`self.Is Valid To Transfer` _index (`local.SourceIndex`) (`local.SourceInventory`)))
      (if _valid
        (return _index))))
  (return -1))

(fn `Get Item Data`
  (params (`Item ID` :type Name))
  (returns (`Item Data` :type "/Game/Systems/Items/Data/Struct/FItemDataStruct Structure"))
  (bind _returnvalue (`|GetDataTableRow` "/Game/Systems/Items/Data/ItemData.ItemData" `Item ID`)
    (:`then`
      (return _returnvalue))))

(fn `Is Valid To Transfer`
  (params (`Destination Index` :type Integer) (`Source Index` :type Integer) (`Source Inventory` :type "/Game/Systems/Inventory/Components/BPC_MasterInventorySystem Object Reference"))
  (returns (Valid :type Boolean))
  (bind ((`AcceptableType_24_E53EA5644608A1B5A3EAB48B1BA9521B` _acceptabletype)) (break `/Game/Systems/Inventory/Slots/Structs/FSlotStruct` (`|GetArrayItem` (`self.Content`) (`local.Destination Index`))))
  (bind ((`Type_26_94813CD2456311DBC7C2D890F9F31D24` _type)) (break `/Game/Systems/Items/Data/Struct/FItemDataStruct` (`self.Get Item Data` (`.Item_26_E76130004EA97320794B31AFED0241D9` (break `/Game/Systems/Inventory/Slots/Structs/FSlotStruct` (`|GetArrayItem` (`/Game/Systems/Inventory/Components/BPC_MasterInventorySystem.Content` (`local.Source Inventory`)) (`local.Source Index`)))))))
  (`KismetSystemLibrary.PrintString` (`KismetStringLibrary.Concat_StrStr` "Destination acceptable type: " (`|GetEnumeratorNameAsString` _acceptabletype) " Source  type:  " (`|GetEnumeratorNameAsString` _type)))
  (return (and (or (!= `Destination Index` `Source Index`) (!= `Source Inventory` self)) (or (`|EnumEquality` _acceptabletype _type) (`|EnumEquality` _acceptabletype "NewEnumerator3")))))

(fn `IsSlotEmpty`
  (params (Index :type Integer) (Inventory :type "/Game/Systems/Inventory/Components/BPC_MasterInventorySystem Object Reference"))
  (returns (IsEmpty :type Boolean))
  (return (`.IsEmpty_10_FE7A134C4724E51CB84AA3B236CF5534` (break `/Game/Systems/Inventory/Slots/Structs/FSlotStruct` (`|GetArrayItem` (`/Game/Systems/Inventory/Components/BPC_MasterInventorySystem.Content` Inventory) Index)))))

(fn `Remove From Slot`
  (params (`Tatget Slot` :type Integer))
  (returns (Item :type Name) (Success :type Boolean))
  (locals (`Local Item` :type Name))
  (bind _output (`|GetArrayItem` (`self.Content`) `Tatget Slot`))
  (bind (_isempty _item) (break `/Game/Systems/Inventory/Slots/Structs/FSlotStruct` _output))
  (if _isempty
    (return "None" true)
    (else
      (set `local.Local Item` _item) ; Setting a local copy of the item
      (setmembers `/Game/Systems/Inventory/Slots/Structs/FSlotStruct` :`StructRef` _output :`IsEmpty` true :`Item` "None") ; Setting slot as emptyand setting item struckt to null?
      (`self.InventoryUpdated` (`local.Tatget Slot`))
      (return (`local.Local Item`) true) ; Returning previous item
    )))

(fn `Transfer Slots`
  (params (`Destination Index` :type Integer) (`Source Index` :type Integer) (`Source Inventory` :type "/Game/Systems/Inventory/Components/BPC_MasterInventorySystem Object Reference"))
  (returns (Success :type Boolean))
  (locals (LocalItem :type "/Game/Systems/Items/Data/Struct/FItemDataStruct Structure"))
  (bind _isempty (`self.IsSlotEmpty` `Source Index` `Source Inventory`))
  (if _isempty
    (return false)
    (else
      (bind _valid (`self.Is Valid To Transfer` (`local.Destination Index`) (`local.Source Index`) (`local.Source Inventory`)))
      (if _valid
        (bind (_item _success) (`self.Remove From Slot` (`local.Source Inventory`) (`local.Source Index`)))
        (if _success
          (bind (_item_2 _success_2) (`self.Remove From Slot` (`local.Destination Index`)))
          (if _success_2
            (`self.Add To Slot` (`local.Source Inventory`) (`local.Source Index`) _item_2)
            (`self.Add To Slot` (`local.Destination Index`) _item)
            (return true)))
        (else
          (return false))))))

(fn `TransferItem`
  (params (SourceIndex :type Integer) (SourceInventory :type "/Game/Systems/Inventory/Components/BPC_MasterInventorySystem Object Reference"))
  (returns (Success :type Boolean))
  (bind _slotindex (`self.FindSuitableSlot` SourceIndex SourceInventory))
  (if (>= _slotindex 0)
    (bind _success (`self.Transfer Slots` _slotindex (`local.SourceIndex`) (`local.SourceInventory`)))
    (return _success)
    (else
      (return false))))

(fn `UseItem`
  (params (ContentId :type Integer))
  (bind _returnvalue (`|GetDataTableRow` "/Game/Systems/Items/Data/ItemData.ItemData" (`.Item_26_E76130004EA97320794B31AFED0241D9` (break `/Game/Systems/Inventory/Slots/Structs/FSlotStruct` (`|GetArrayItem` (`self.Content`) ContentId))))
    (:`then`
      (bind ((`ItemClass_23_561B5055463ABFA66C29908BA060C37A` _itemclass)) (break `/Game/Systems/Items/Data/Struct/FItemDataStruct` _returnvalue))
      (if (`KismetSystemLibrary.DoesClassImplementInterface` _itemclass "/Game/Interfaces/BI_Consumable.BI_Consumable_C")
        (bind _asbp_first_person_character (cast `/Game/FirstPerson/Blueprints/BP_FirstPersonCharacter` (`self.GetOwner`)))
        (bind _returnvalue_2 (`|SpawnActorFromClass` _itemclass (`KismetMathLibrary.MakeTransform` (`KismetMathLibrary.MakeVector` 0.0)) "AlwaysSpawn" "MultiplyWithRoot" null null))
        (`self.Remove From Slot` (`local.ContentId`))
        (bind _success (message `/Game/Interfaces/BI_Consumable.Consume` _returnvalue_2 _asbp_first_person_character))
        (if _success
          (`Actor.K2_DestroyActor` _returnvalue_2))))))