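; Player inventory component that handles picking up, dropping, counting and consuming items in a slot array, one item per slot.
; BeginPlay caches the first-person character's HUD and initializes the player menu.
; Pickups fill the first empty slot; drops spawn the data-table item class in a random cone ahead of the owner, both showing HUD messages.
; TryUseItems verifies every required quantity before removing any items.
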(event `self.ReceiveBeginPlay`
  (bind _asbp_first_person_character (cast `/Game/FirstPerson/Blueprints/BP_FirstPersonCharacter` (`self.GetOwner`)))
  (bind _asbp_first_person_player_controller (cast `/Game/FirstPerson/Blueprints/BP_FirstPersonPlayerController` (`Pawn.GetController` _asbp_first_person_character)))
  (bind _asdwarf_hud (cast `/Game/Widgets/HUD/DwarfHUD` (`PlayerController.GetHUD` _asbp_first_person_player_controller)))
  (set `self.DwarfHUD` (`|ConvertAsset` _asdwarf_hud))
  (`parent.ReceiveBeginPlay`)
  (`/Game/Widgets/HUD/DwarfHUD.InitializePlayerMenu` _asdwarf_hud))

(fn `Drop Item`
  (params (`Item Slot` :type Integer))
  (locals (`Slot Struct` :type "/Game/Systems/Inventory/Slots/Structs/FSlotStruct Structure") (`Item Struct` :type "/Game/Systems/Items/Data/Struct/FItemStruct Structure"))
  (bind (_item _success) (`self.Remove From Slot` `Item Slot`))
  (if _success
    (bind _returnvalue (`|GetDataTableRow` "/Game/Systems/Items/Data/ItemData.ItemData" _item)
      (:`then`
        (`self.Spawn Item` _item)
        (`/Game/Widgets/HUD/DwarfHUD.ShowInfoMessage` (`|ConvertAsset` (`self.DwarfHud`)) (`KismetStringLibrary.Concat_StrStr` "Dropped " (`KismetTextLibrary.Conv_TextToString` (`.DisplayedName_40_78255BC3428C1EA3F5B408B4514736C4` (break `/Game/Systems/Items/Data/Struct/FItemDataStruct` _returnvalue)))))))))

(fn `FindItem`
  (params (ItemId :type Name) (Quantity :type Integer) (Destroy :type Boolean))
  (returns (`Enough?` :type Boolean))
  (locals (SummaryQuantity :type Integer) (ItemIds :type "Array of Integer") (Enough :type Boolean))
  (for (_array_element _array_index) (`self.Content`)
    (if (== (`local.ItemId`) (`.Item_26_E76130004EA97320794B31AFED0241D9` (break `/Game/Systems/Inventory/Slots/Structs/FSlotStruct` _array_element)))
      (`KismetArrayLibrary.Array_Add` (`local.ItemIds`) _array_index)
      (`/Engine/EditorBlueprintResources/StandardMacros.IncrementInt` (`local.SummaryQuantity`)
        (:`  `
          (bind _output_get (set `local.Enough` (== (`local.SummaryQuantity`) (`local.Quantity`))))
          (if _output_get
            (break))))))
  (if (and (`local.Destroy`) (`local.Enough`))
    (for _array_element_2 (`local.ItemIds`)
      (bind (_item _success) (`self.Remove From Slot` _array_element_2))
      (if (not _success)
        (return false))))
  (return (`local.Enough`)))

(fn `FindItemQuantity`
  (params (`Item ID` :type Name))
  (returns (Quantity :type Integer))
  (locals (`Quantity ` :type Integer))
  (for _array_element (`self.Content`)
    (bind (_isempty _item) (break `/Game/Systems/Inventory/Slots/Structs/FSlotStruct` _array_element))
    (if (and (not _isempty) (== _item (`local.Item ID`)))
      (`/Engine/EditorBlueprintResources/StandardMacros.IncrementInt` (`local.Quantity `))))
  (return (`local.Quantity `)))

(fn `FindSlot`
  (returns (`Slot Id` :type Integer))
  (locals (Index :type Integer))
  (for (_array_element _array_index) (`self.Content`)
    (set `local.Index` _array_index)
    (if (`.IsEmpty_10_FE7A134C4724E51CB84AA3B236CF5534` (break `/Game/Systems/Inventory/Slots/Structs/FSlotStruct` _array_element))
      (return (`local.Index`))))
  (return -1))

(fn `Get Drop Location`
  (returns (Location :type "Vector Structure"))
  (bind _returnvalue (`self.GetOwner`))
  (return (+ (`Actor.K2_GetActorLocation` _returnvalue) (* (`KismetMathLibrary.RandomUnitVectorInConeInDegrees` (`Actor.GetActorForwardVector` _returnvalue) 30.0) 100.0))))

(fn `Get Item Quantity`
  (params (`Item ID` :type Name))
  (returns (Quantity :type Integer))
  (bind _quantity (`self.FindItemQuantity` `Item ID`))
  (return _quantity))

(fn `PickUpItem`
  (params (ItemName :type Name))
  (returns (Success :type Boolean))
  (bind _slot_id (`self.FindSlot`))
  (if (> _slot_id -1)
    (`self.CollectED`)
    (`self.Add To Slot` _slot_id (`local.ItemName`))
    (bind _returnvalue (`|GetDataTableRow` "/Game/Systems/Items/Data/ItemData.ItemData" (`local.ItemName`))
      (:`then`
        (`/Game/Widgets/HUD/DwarfHUD.ShowInfoMessage` (`|ConvertAsset` (`self.DwarfHud`)) (`KismetStringLibrary.Concat_StrStr` "Picked up " (`KismetTextLibrary.Conv_TextToString` (`.DisplayedName_40_78255BC3428C1EA3F5B408B4514736C4` (break `/Game/Systems/Items/Data/Struct/FItemDataStruct` _returnvalue)))))
        (return true)))
    (else
      (return false))))

(fn `Spawn Item`
  (params (ItemId :type Name))
  (bind _returnvalue (`|SpawnActorFromClass` (`.ItemClass_23_561B5055463ABFA66C29908BA060C37A` (break `/Game/Systems/Items/Data/Struct/FItemDataStruct` (`self.Get Item Data` ItemId))) (`KismetMathLibrary.MakeTransform` (`self.Get Drop Location`)) "Undefined" "MultiplyWithRoot" null null))
  (`/Game/Objects/Items/BP_ItemObjectMaster.Change Item Quantity` _returnvalue 1))

(fn `TryUseItems`
  (params (Items :type "Map of Name to Integer"))
  (returns (`Enough?` :type Boolean))
  (locals (IsEnough :type Boolean :default true) (Array :type Boolean))
  (bind _keys (`BlueprintMapLibrary.Map_Keys` Items))
  (for _array_element _keys
    (bind _enough_ (`self.FindItem` _array_element (`BlueprintMapLibrary.Map_Find` (`local.Items`) _array_element)))
    (bind _output_get (set `local.IsEnough` _enough_))
    (if (not _output_get)
      (break)))
  (if (`local.IsEnough`)
    (bind _keys_2 (`BlueprintMapLibrary.Map_Keys` (`local.Items`)))
    (for _array_element_2 _keys_2
      (`self.FindItem` _array_element_2 (`BlueprintMapLibrary.Map_Find` (`local.Items`) _array_element_2) true)))
  (return (`local.IsEnough`)))