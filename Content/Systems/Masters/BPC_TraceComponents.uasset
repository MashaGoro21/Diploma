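; BPC_TraceComponents is a master component for periodic camera traces on the first-person player character.
; On BeginPlay it caches the owning BP_FirstPersonCharacter and starts a looping timer.
; While player input is enabled, each tick of that timer passes the camera location and a length-based end point to TraceEvent, an empty hook.
; TraceTypeFunc provides a sphere trace on the Visibility channel but is not called here.
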(event `self.ReceiveBeginPlay`
  (bind _asbp_first_person_character (cast `/Game/FirstPerson/Blueprints/BP_FirstPersonCharacter` (`self.GetOwner`)))
  (set `self.Player` _asbp_first_person_character)
  (`KismetSystemLibrary.K2_SetTimerDelegate` (delegate `TimerEvent`) 0.1 true true))

(event `TimerEvent`
  (bind _player (`self.Player`))
  (if (`/Game/FirstPerson/Blueprints/BP_FirstPersonCharacter.IsInputEnabled` (`self.Player`))
    (bind _end (`/Game/FirstPerson/Blueprints/BP_FirstPersonCharacter.SetTraceLength` _player (`self.TraceLength`)))
    (if (`/Game/FirstPerson/Blueprints/BP_FirstPersonCharacter.IsInputEnabled` (`self.Player`))
      (`self.TraceEvent` (`SceneComponent.K2_GetComponentLocation` (`/Game/FirstPerson/Blueprints/BP_FirstPersonCharacter.FirstPersonCamera` _player)) _end))))

(event `TraceEvent`
  (params (Start :type "Vector Structure") (End :type "Vector Structure")))

(fn `TraceTypeFunc`
  (params (Start :type "Vector Structure") (End :type "Vector Structure") (Radius :type "Float (double-precision)"))
  (`KismetSystemLibrary.SphereTraceSingle` Start End Radius "TraceTypeQuery1"))