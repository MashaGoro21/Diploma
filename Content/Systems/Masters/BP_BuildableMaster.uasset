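; Master Blueprint for buildable world objects that the player turns into a target actor when an item check passes.
; Highlighting pushes a popup of required items onto the modal UI layer.
; Interaction marks it built, plays a sound, then spawns ObjectToBuild and destroys itself.
; Built state is keyed by actor path, written to an archive save map and loaded from IsBuildedMap, rebuilding on BeginPlay.
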(event `self.ReceiveBeginPlay`
  (bind _returnvalue (`KismetSystemLibrary.GetPathName` self))
  (`parent.ReceiveBeginPlay`)
  (bind _returnvalue_2 (`|CreateWidget` "/Game/Widgets/WB_BuildPopup.WB_BuildPopup_C"))
  (set `self.BuildPopup` _returnvalue_2)
  (bind _asbp_game_instance (cast `/Game/Systems/Save/BP_GameInstance` (`GameplayStatics.GetGameInstance`)))
  (bind _savegameref (`/Game/Systems/Save/BP_GameInstance.SaveGameRef` _asbp_game_instance))
  (set `self.SaveGameRef` _savegameref)
  (bind _isbuildedmap (`/Game/Systems/Save/BP_SaveGame.IsBuildedMap` _savegameref))
  (if (not (`BlueprintMapLibrary.Map_Contains` _isbuildedmap _returnvalue))
    (`BlueprintMapLibrary.Map_Add` _isbuildedmap _returnvalue (`self.IsBuilded`)))
  (message `/Game/Systems/Save/BPI_Persistence.RequestLoad` (`GameplayStatics.GetGameInstance`) self)
  (if (`self.IsBuilded`)
    (`self.BuildObject`)))

(event `/Game/Interfaces/BI_Interactable.Interaction`
  (params (`Player ` :type "/Game/FirstPerson/Blueprints/BP_FirstPersonCharacter Object Reference"))
  (bind _buildingsound (`self.BuildingSound`))
  (if (not (`self.IsBuilded`))
    (bind _enough_ (`/Game/FirstPerson/Blueprints/BP_FirstPersonCharacter.CheckItems` `Player ` (`self.Items`)))
    (if _enough_
      (`self.SetObjectBuilded`)
      (`AudioComponent.Play` _buildingsound 0.0)
      (`KismetSystemLibrary.Delay` (`SoundBase.Duration` (`AudioComponent.Sound` _buildingsound)))
      (`self.BuildObject`))))

(event `/Game/Systems/Save/BPI_Saveable.LoadData`
  (params (SaveGameRef :type "/Game/Systems/Save/BP_SaveGame Object Reference"))
  (set `self.IsBuilded` (`BlueprintMapLibrary.Map_Find` (`/Game/Systems/Save/BP_SaveGame.IsBuildedMap` SaveGameRef) (`KismetSystemLibrary.GetPathName` self))))

(fn `BuildObject`
  (`|SpawnActorFromClass` (`self.ObjectToBuild`) (`SceneComponent.GetRelativeTransform` (`self.Scene`)) "Undefined" "MultiplyWithRoot" null null)
  (`self.K2_DestroyActor`))

(fn `SetHighlightStatus`
  (params (IsSelected :type Boolean) (Material :type "MaterialInterface Object Reference"))
  (bind _returnvalue (`GameplayStatics.GetPlayerController` 0))
  (`parent.SetHighlightStatus` IsSelected Material)
  (if IsSelected
    (`/Game/Widgets/WB_BuildPopup.SetItemsView` (`self.BuildPopup`) (`self.Items`))
    (`/Game/Widgets/WidgetManager/BPFL_UI.PushWidgetToLayer` _returnvalue (struct :`TagName` "UI.Layer.Modal") (`self.BuildPopup`))
    (else
      (`/Game/Widgets/WidgetManager/BPFL_UI.PopContentFromLayer` _returnvalue (struct :`TagName` "UI.Layer.Modal")))))

(fn `SetObjectBuilded`
  (bind _output_get (set `self.IsBuilded` true))
  (`BlueprintMapLibrary.Map_Add` (`/Game/Systems/Save/BP_SaveGame.IsBuildedMapArchive` (`self.SaveGameRef`)) (`KismetSystemLibrary.GetPathName` self) _output_get))

(fn `UserConstructionScript`
  (`parent.UserConstructionScript`))