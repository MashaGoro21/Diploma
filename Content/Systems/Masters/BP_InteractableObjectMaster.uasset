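; Base actor for interactable objects, providing selection highlighting and stub interaction events.
; HighlightObject calls SetHighlightStatus, which on a state change toggles an overlay material on the Meshes array and shows or hides KeyWidget.
; BeginPlay fills the array through SetMeshes (only MainMesh here), destroys the Box component and binds OnDestroyed to clear the highlight.
; Interaction only prints the player's name and React is empty.
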(event `self.ReceiveBeginPlay`
  (`self.SetMeshes`)
  (add `self.OnDestroyed` (delegate `OnDestroyed_Event`))
  (`ActorComponent.K2_DestroyComponent` (`self.Box`)))

(event `OnDestroyed_Event` :!signature `self.OnDestroyed`
  (params (DestroyedActor :type "Actor Object Reference"))
  (`self.SetHighlightStatus` false))

(event `/Game/Interfaces/BI_Interactable.HighlightObject`
  (params (IsSelected :type Boolean))
  (`self.SetHighlightStatus` IsSelected (`self.OverlayMaterial`)))

(event `/Game/Interfaces/BI_Interactable.Interaction`
  (params (`Player ` :type "/Game/FirstPerson/Blueprints/BP_FirstPersonCharacter Object Reference"))
  (`KismetSystemLibrary.PrintString` (`KismetSystemLibrary.GetDisplayName` `Player `)))

(event `/Game/Interfaces/BI_Reactive.React`)

(fn `SetHighlightStatus`
  (params (IsSelected :type Boolean) (Material :type "MaterialInterface Object Reference"))
  (if (!= IsSelected (`self.Selected?`))
    (set `self.Selected?` (`local.IsSelected`))
    (for _array_element (`self.Meshes`)
      (if (`self.Selected?`)
        (`MeshComponent.SetOverlayMaterial` _array_element (`local.Material`))
        (else
          (`MeshComponent.SetOverlayMaterial` _array_element null))))
    (`SceneComponent.SetHiddenInGame` (`self.KeyWidget`) (not (`self.Selected?`)) false)))

(fn `SetMeshes`
  (set `self.Meshes` (`|MakeArray` (`self.MainMesh`) :!type "MeshComponent Object Reference")))

(fn `UserConstructionScript`)