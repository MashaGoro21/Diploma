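; BP_MasterStation is a base interactable station with its own inventory and UI widget.
; Interaction hides the player, disables their input, blends the view to the station and pushes the widget onto the game menu layer, while Interact or Quit reverses this.
; Open and close calls follow each transition.
; Helpers create the inventory-bound widget and fill child actors with item classes from a data table; the inventory update handler is empty here.
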(event `self.ReceiveBeginPlay`
  (message `/Game/Interfaces/BI_InventoryOwner.SetStationInventory` (`self.MainWidget`) (`self.StationInventory`))
  (`self.SetMeshes`)
  (add `/Game/Systems/Inventory/Components/BPC_MasterInventorySystem.InventoryUpdated` (`self.StationInventory`) (delegate `OnInventoryUpdated`)))

(event `OnInventoryUpdated`
  (params (SlotId :type Integer)))

(event `/Game/Interfaces/BI_Interactable.Interaction`
  (params (`Player ` :type "/Game/FirstPerson/Blueprints/BP_FirstPersonCharacter Object Reference"))
  (`self.Player`
    (:`then`
      _)
    (:`else`
      (bind _output_get (set `self.Player` `Player `))))
  (`self.Player Controller`
    (:`then`
      _)
    (:`else`
      (set `self.Player Controller` (`Pawn.GetLocalViewingPlayerController` _output_get))))
  (`self.StartInspection`))

(event `StartInspection`
  (`/Game/FirstPerson/Blueprints/BP_FirstPersonCharacter.SetInputStatus` (`self.Player`) false)
  (`/Game/FirstPerson/Blueprints/BP_FirstPersonCharacter.ChangePlayerVisibility` (`self.Player`) false)
  (`PlayerController.SetViewTargetWithBlend` (`self.Player Controller`) self (`self.BlendTime`) "VTBlend_Linear" 0.0 false)
  (`KismetSystemLibrary.Delay` (`self.BlendTime`))
  (`self.EnableInput` (`self.Player Controller`))
  (bind _widget (`/Game/Widgets/WidgetManager/BPFL_UI.PushWidgetToLayer` (`self.Player Controller`) (struct :`TagName` "UI.Layer.GameMenu") (`self.MainWidget`)))
  (`/Game/Widgets/WidgetManager/BPFL_UI.FocusModal` (`self.Player Controller`) _widget)
  (`self.OnOpen`))

(event `EnhancedInput|/Game/FirstPerson/Input/Actions/IA_Interact`
  (params (ActionValue :type Boolean) (ElapsedSeconds :type "Float (double-precision)") (TriggeredSeconds :type "Float (double-precision)") (InputAction :type "InputAction Object Reference" :default "/Game/FirstPerson/Input/Actions/IA_Interact.IA_Interact"))
  (:`Triggered`
    (`self.QuitInspection` :!label _label)))

(event `EnhancedInput|/Game/FirstPerson/Input/Actions/IA_Quit`
  (params (ActionValue :type Boolean) (ElapsedSeconds :type "Float (double-precision)") (TriggeredSeconds :type "Float (double-precision)") (InputAction :type "InputAction Object Reference" :default "/Game/FirstPerson/Input/Actions/IA_Quit.IA_Quit"))
  (:`Triggered`
    (goto _label)))

(event `QuitInspection`
  (`/Game/Widgets/WidgetManager/BPFL_UI.PopContentFromLayer` (`self.Player Controller`) (struct :`TagName` "UI.Layer.GameMenu"))
  (`self.DisableInput` (`self.Player Controller`))
  (`PlayerController.SetViewTargetWithBlend` (`self.Player Controller`) (`self.Player`) (`self.BlendTime`) "VTBlend_Linear" 0.0 false)
  (`KismetSystemLibrary.Delay` (`self.BlendTime`))
  (`/Game/FirstPerson/Blueprints/BP_FirstPersonCharacter.SetInputStatus` (`self.Player`) true)
  (`/Game/FirstPerson/Blueprints/BP_FirstPersonCharacter.ChangePlayerVisibility` (`self.Player`) true)
  (`/Game/Widgets/WidgetManager/BPFL_UI.FocusGame` (`self.Player Controller`))
  (`self.OnClose`))

(fn `SetItem`
  (params (Item :type Name) (ChildActor :type "ChildActorComponent Object Reference"))
  (bind _returnvalue (`|GetDataTableRow` "/Game/Systems/Items/Data/ItemData.ItemData" Item)
    (:`then`
      (`ChildActorComponent.SetChildActorClass` (`local.ChildActor`) (`.ItemClass_23_561B5055463ABFA66C29908BA060C37A` (break `/Game/Systems/Items/Data/Struct/FItemDataStruct` _returnvalue)))
      (message `/Game/Interfaces/BI_Item.ChangeState` (`ChildActorComponent.ChildActor` (`local.ChildActor`)) false))
    (:`RowNotFound`
      (`ChildActorComponent.SetChildActorClass` (`local.ChildActor`) null))))

(fn `SetWidget`
  (params (Widget :type "UserWidget Class Reference"))
  (bind _returnvalue (`|CreateWidget` Widget (`GameplayStatics.GetPlayerController` 0)))
  (bind _output_get (set `self.MainWidget` _returnvalue))
  (message `/Game/Interfaces/BI_InventoryOwner.SetStationInventory` _output_get (`self.StationInventory`)))

(fn `UserConstructionScript`)