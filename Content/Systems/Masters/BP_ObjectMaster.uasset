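; BP_ObjectMaster is a master object Blueprint that switches its mesh to physics simulation once it no longer touches the voxel world.
; React nudges the Box up and back down, apparently to refresh overlaps, then checks it for VoxelWorld actors.
; With no overlap and a Movable mesh, it calls SetPhysicsStatus, which enables simulation and destroys the Box, so later React calls do nothing.
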(event `SetPhysicsStatus`
  (params (Status :type Boolean))
  (bind _output_get (set `self.Is Physics Simulating` Status))
  (`PrimitiveComponent.SetSimulatePhysics` (`self.MainMesh`) _output_get)
  (if (`self.Is Physics Simulating`)
    (`ActorComponent.K2_DestroyComponent` (`self.Box`))))

(event `/Game/Interfaces/BI_Reactive.React`
  (`/Engine/EditorBlueprintResources/StandardMacros.IsValid` (`self.Box`)
    (:`Is Valid`
      (`SceneComponent.K2_AddRelativeLocation` (`self.Box`) (0.0 0.0 1.0) false false)
      (`SceneComponent.K2_AddRelativeLocation` (`self.Box`) (0.0 0.0 -1.0) false false)
      (if (and (== (`SceneComponent.Mobility` (`self.MainMesh`)) 2) (== (`KismetArrayLibrary.Array_Length` (`PrimitiveComponent.GetOverlappingActors` (`self.Box`) "/Script/Voxel.VoxelWorld")) 0))
        (`self.SetPhysicsStatus` true)))))

(fn `UserConstructionScript`)