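; BP_UIManager manages UI widgets, here the build popup that shows a list of items.
; DisplayBuildPopUp lazily creates WB_BuildPopup on first show, caches it, adds it to the viewport and passes it the items to display.
; Hiding removes the cached widget from its parent, so later shows reuse the same instance.
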(fn `DisplayBuildPopUp`
  (params (Items :type "Map of Name to Integer") (`Display?` :type Boolean))
  (bind _buildpopup (`self.BuildPopup`))
  (if `Display?`
    (`/Engine/EditorBlueprintResources/StandardMacros.IsValid` (`self.BuildPopup`)
      (:`Is Valid`
        _)
      (:`Is Not Valid`
        (bind _returnvalue (`|CreateWidget` "/Game/Widgets/WB_BuildPopup.WB_BuildPopup_C"))
        (set `self.BuildPopup` _returnvalue)))
    (`UserWidget.AddToViewport` (`self.BuildPopup`) 0)
    (`/Game/Widgets/WB_BuildPopup.SetItemsView` (`self.BuildPopup`) (`local.Items`))
    (else
      (`/Engine/EditorBlueprintResources/StandardMacros.IsValid` _buildpopup
        (:`Is Valid`
          (`Widget.RemoveFromParent` _buildpopup))))))