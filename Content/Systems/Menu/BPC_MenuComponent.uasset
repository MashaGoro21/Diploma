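; BPC_MenuComponent is a component that shows the pause menu and death screen for the first-person player.
; On BeginPlay it creates both widgets and binds the player character's death event to showing the death screen.
; The quit input opens the pause menu; both screens are pushed to the UI.Layer.Menu layer as focused modals that pause the game and take UI-only input.
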(event `self.ReceiveBeginPlay`
  (set `self.PlayerController` (`GameplayStatics.GetPlayerController` 0))
  (bind _returnvalue (`|CreateWidget` "/Game/Systems/Menu/WB_PauseMenu.WB_PauseMenu_C" (`self.PlayerController`)))
  (set `self.PauseMenuWidget` _returnvalue)
  (bind _returnvalue_2 (`|CreateWidget` "/Game/Systems/Menu/WB_DeathWidget.WB_DeathWidget_C" (`self.PlayerController`)))
  (set `self.DeathWidget` _returnvalue_2)
  (bind _asbp_first_person_character (cast `/Game/FirstPerson/Blueprints/BP_FirstPersonCharacter` (`GameplayStatics.GetPlayerPawn` 0)))
  (bind _output_get (set `self.Player` _asbp_first_person_character))
  (add `/Game/FirstPerson/Blueprints/BP_FirstPersonCharacter.ED_Died` _output_get (delegate `ShowDeathWidget`)))

(event `ShowDeathWidget`
  (bind _widget (`/Game/Widgets/WidgetManager/BPFL_UI.PushWidgetToLayer` (`self.PlayerController`) (struct :`TagName` "UI.Layer.Menu") (`self.DeathWidget`)))
  (`/Game/Widgets/WidgetManager/BPFL_UI.FocusModal` (`self.PlayerController`) _widget true true true))

(event `EnhancedInput|/Game/FirstPerson/Input/Actions/IA_Quit`
  (params (ActionValue :type Boolean) (ElapsedSeconds :type "Float (double-precision)") (TriggeredSeconds :type "Float (double-precision)") (InputAction :type "InputAction Object Reference" :default "/Game/FirstPerson/Input/Actions/IA_Quit.IA_Quit"))
  (:`Completed`
    (`self.ShowWidget` (`self.PauseMenuWidget`))))

(fn `ShowWidget`
  (params (Widget :type "UserWidget Object Reference"))
  (bind _widget (`/Game/Widgets/WidgetManager/BPFL_UI.PushWidgetToLayer` (`self.PlayerController`) (struct :`TagName` "UI.Layer.Menu") Widget))
  (`/Game/Widgets/WidgetManager/BPFL_UI.FocusModal` (`self.PlayerController`) _widget true true true))