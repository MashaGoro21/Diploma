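; BP_EndGameObject is an interactable actor that brings up the end-game screen.
; Its Interaction event casts the interacting player's controller to BP_FirstPersonPlayerController, then creates a WB_EndGame widget owned by that controller and adds it to the viewport.
; The other event stubs are disabled and the construction script only calls its parent.
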(event `/Game/Interfaces/BI_Interactable.Interaction`
  (params (`Player ` :type "/Game/FirstPerson/Blueprints/BP_FirstPersonCharacter Object Reference"))
  (bind _asbp_first_person_player_controller (cast `/Game/FirstPerson/Blueprints/BP_FirstPersonPlayerController` (`Pawn.GetController` `Player `)))
  (bind _returnvalue (`|CreateWidget` "/Game/Widgets/WB_EndGame.WB_EndGame_C" _asbp_first_person_player_controller))
  (`UserWidget.AddToViewport` _returnvalue 0))

(fn `UserConstructionScript`
  (`parent.UserConstructionScript`))