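; BP_NiagaraControlSystem is a helper Blueprint that drives a Niagara effect and its debris material.
; ActiveEffect assigns a given system asset to the NiagaraEffect component, resetting overrides, then moves it to a position and activates it.
; ChangeTexture creates a dynamic instance of M_Debris_Master with the given texture and passes it to ChangeMaterial, which sets the effect's DynamicMaterial variable.
; The event graph and construction script are empty, so these functions rely on external callers.
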(fn `ActiveEffect`
  (params (NiagaraEffect :type "NiagaraSystem Object Reference") (Position :type "Vector Structure"))
  (`NiagaraComponent.SetAsset` (`self.NiagaraEffect`) NiagaraEffect true)
  (`SceneComponent.K2_SetWorldLocation` (`self.NiagaraEffect`) (`local.Position`) false false)
  (`ActorComponent.Activate` (`self.NiagaraEffect`) true))

(fn `ChangeMaterial`
  (params (Material :type "MaterialInterface Object Reference"))
  (`NiagaraComponent.SetVariableMaterial` (`self.NiagaraEffect`) "DynamicMaterial" Material))

(fn `ChangeTexture`
  (params (Texture :type "Texture2D Object Reference"))
  (bind _returnvalue (`KismetMaterialLibrary.CreateDynamicMaterialInstance` "/Game/Assets/Materials/FX/M_Debris_Master.M_Debris_Master"))
  (bind _output_get (set `self.Material` _returnvalue))
  (`MaterialInstanceDynamic.SetTextureParameterValue` _output_get "Texture" Texture)
  (`self.ChangeMaterial` (`self.Material`)))

(fn `UserConstructionScript`)