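; Actor component that holds the first-person character's collection of notes and opens the notes display on the HUD.
; AddNote looks up a row in DT_Notes by name and appends the row data to the Notes array.
; The IA_Notes input opens the player HUD's notes view at index 0 through NotesMenu, which accepts any index.
; It requests a load from the game instance on BeginPlay and copies Notes to and from the save game.
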(event `self.ReceiveBeginPlay`
  (bind _asbp_first_person_character (cast `/Game/FirstPerson/Blueprints/BP_FirstPersonCharacter` (`self.GetOwner`)))
  (set `self.Player` _asbp_first_person_character)
  (message `/Game/Systems/Save/BPI_Persistence.RequestLoad` (`GameplayStatics.GetGameInstance`) self))

(event `EnhancedInput|/Game/FirstPerson/Input/Actions/IA_Notes`
  (params (ActionValue :type Boolean) (ElapsedSeconds :type "Float (double-precision)") (TriggeredSeconds :type "Float (double-precision)") (InputAction :type "InputAction Object Reference" :default "/Game/FirstPerson/Input/Actions/IA_Notes.IA_Notes"))
  (:`Completed`
    (`self.NotesMenu` 0)))

(event `NotesMenu`
  (params (Index :type Integer))
  (`/Game/Widgets/HUD/DwarfHUD.DisplayNotes` (`/Game/FirstPerson/Blueprints/BP_FirstPersonCharacter.HUD` (`self.Player`)) Index))

(event `/Game/Systems/Save/BPI_Saveable.LoadData`
  (params (SaveGameRef :type "/Game/Systems/Save/BP_SaveGame Object Reference"))
  (set `self.Notes` (`/Game/Systems/Save/BP_SaveGame.Notes` SaveGameRef)))

(event `/Game/Systems/Save/BPI_Saveable.SaveData`
  (params (SaveGameRef :type "/Game/Systems/Save/BP_SaveGame Object Reference"))
  (set `/Game/Systems/Save/BP_SaveGame.Notes` (`self.Notes`) SaveGameRef))

(fn `AddNote`
  (params (Note :type Name))
  (returns (Index :type Integer))
  (bind _returnvalue (`|GetDataTableRow` "/Game/Systems/Notes/DT_Notes.DT_Notes" Note)
    (:`then`
      (bind _returnvalue_2 (`KismetArrayLibrary.Array_Add` (`self.Notes`) _returnvalue))
      (return _returnvalue_2))))