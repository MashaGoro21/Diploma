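; BP_NoteItem is a note pickup actor that adds its note to the interacting player's notes inventory.
; On Interaction it passes its Note to the player's BPCNotesInventory, calls NotesMenu with the result of AddNote, then destroys itself.
; GetNotesNames returns the row names of the DT_Notes data table.
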(event `/Game/Interfaces/BI_Interactable.Interaction`
  (params (`Player ` :type "/Game/FirstPerson/Blueprints/BP_FirstPersonCharacter Object Reference"))
  (bind _bpc_notesinventory (`/Game/FirstPerson/Blueprints/BP_FirstPersonCharacter.BPC_NotesInventory` `Player `))
  (bind _index (`/Game/Systems/Notes/BPC_NotesInventory.AddNote` _bpc_notesinventory (`self.Note`)))
  (`/Game/Systems/Notes/BPC_NotesInventory.NotesMenu` _bpc_notesinventory _index)
  (`self.K2_DestroyActor`))

(fn `GetNotesNames`
  (returns (Notes :type "Array of Name"))
  (bind _outrownames (`DataTableFunctionLibrary.GetDataTableRowNames` "/Game/Systems/Notes/DT_Notes.DT_Notes"))
  (return _outrownames))

(fn `UserConstructionScript`
  (`parent.UserConstructionScript`))