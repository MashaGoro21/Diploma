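; BP_GoblinBox is a trade station that swaps the item placed in it for a reward.
; Inventory updates refresh the goblin widget, set the displayed child actor item, and drive a Timeline that rotates a scene component according to whether the slot is empty.
; When the widget fires its offer event, StartTrade scans DT_GoblinTradeData for rows matching slot 0's item and replaces it with that row's reward.
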(event `self.ReceiveBeginPlay`
  (`parent.ReceiveBeginPlay`)
  (bind _aswb_golbin_widget (cast `/Game/Systems/Puzzles/Widgets/WB_GolbinWidget` (`self.MainWidget`)))
  (bind _output_get (set `self.Golbin Widget` _aswb_golbin_widget))
  (add `/Game/Systems/Puzzles/Widgets/WB_GolbinWidget.ED_OffetItem` _output_get (delegate `StartTrade`)))

(event `self.OnInventoryUpdated`
  (params (SlotId :type Integer))
  (bind ((`IsEmpty_10_FE7A134C4724E51CB84AA3B236CF5534` _isempty) (`Item_26_E76130004EA97320794B31AFED0241D9` _item)) (break `/Game/Systems/Inventory/Slots/Structs/FSlotStruct` (`|GetArrayItem` (`/Game/Systems/Inventory/Components/BPC_MasterInventorySystem.Content` (`self.StationInventory`)) SlotId)))
  (message `/Game/Interfaces/BI_InventoryOwner.UpdateInventory` (`self.Golbin Widget`))
  (`/Game/Systems/Puzzles/Widgets/WB_GolbinWidget.InitializeButton` (`self.Golbin Widget`))
  (`self.SetItem` _item (`self.ChildActor`))
  (if _isempty
    (bind (_direction `_новая_дорожка_0`) (`Timeline|Timeline` :!via `Reverse` :!label _label)
      (:`Update`
        (`SceneComponent.K2_SetRelativeRotation` (`self.Scene_0`) (`KismetMathLibrary.MakeRotator` 180.0 (`KismetMathLibrary.Lerp` -50.0 -180.0 `_новая_дорожка_0`) 180.0) false false)))
    (else
      (goto _label))))

(event `StartTrade`
  (bind _stationinventory (`self.StationInventory`))
  (bind _outrownames (`DataTableFunctionLibrary.GetDataTableRowNames` "/Game/Systems/Puzzles/DT_GoblinTradeData.DT_GoblinTradeData"))
  (for _array_element _outrownames
    (bind _returnvalue (`|GetDataTableRow` "/Game/Systems/Puzzles/DT_GoblinTradeData.DT_GoblinTradeData" _array_element)
      (:`then`
        (bind (_item _reward) (break `/Game/Systems/Puzzles/FGoblinTradeStruct` _returnvalue))
        (if (== (`.ItemId_2_D15E650D447F179120E90DBF367FFFF8` (break `/Game/Systems/Items/Data/Struct/FItemStruct` _item)) (`.Item_26_E76130004EA97320794B31AFED0241D9` (break `/Game/Systems/Inventory/Slots/Structs/FSlotStruct` (`|GetArrayItem` (`/Game/Systems/Inventory/Components/BPC_MasterInventorySystem.Content` (`self.StationInventory`))))))
          (`/Game/Systems/Inventory/Components/BPC_MasterInventorySystem.Remove From Slot` _stationinventory 0)
          (`/Game/Systems/Inventory/Components/BPC_MasterInventorySystem.Add To Slot` _stationinventory 0 (`.ItemId_2_D15E650D447F179120E90DBF367FFFF8` (break `/Game/Systems/Items/Data/Struct/FItemStruct` _reward)))
          (message `/Game/Interfaces/BI_InventoryOwner.UpdateInventory` (`self.Golbin Widget`)))))))

(fn `UserConstructionScript`
  (`parent.UserConstructionScript`))