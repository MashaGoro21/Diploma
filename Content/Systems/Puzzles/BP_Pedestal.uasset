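; BP_Pedestal is an inspectable puzzle pedestal that expects a specific item to be placed in its station inventory.
; When a slot updates, it refreshes the UI, passes the placed item to its child actor, and compares it to the required item row.
; A match marks it solved and fires the pedestal-updated dispatcher.
; Starting inspection shows the required item's hint text from the DT_PedestalText data table.
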(event `self.OnInventoryUpdated`
  (params (SlotId :type Integer))
  (bind ((`Item_26_E76130004EA97320794B31AFED0241D9` _item)) (break `/Game/Systems/Inventory/Slots/Structs/FSlotStruct` (`|GetArrayItem` (`/Game/Systems/Inventory/Components/BPC_MasterInventorySystem.Content` (`self.StationInventory`)) SlotId)))
  (message `/Game/Interfaces/BI_InventoryOwner.UpdateInventory` (`self.MainWidget`))
  (`self.SetItem` _item (`self.ChildActor`))
  (bind _output_get (set `self.IsSolved` (== (`.RowName` (break `DataTableRowHandle` (`self.Item`))) _item)))
  (if _output_get
    (`self.ED_PedestalUpdated`)))

(event `self.StartInspection`
  (`parent.StartInspection`)
  (bind _returnvalue (`|GetDataTableRow` "/Game/Systems/Puzzles/DT_PedestalText.DT_PedestalText" (`.RowName` (break `DataTableRowHandle` (`self.Item`))))
    (:`then`
      (message `/Game/Interfaces/BI_WidgetSetup.SetText` (`self.MainWidget`) (`.HintText_2_DB6DEB61445066681522499A30FC74C4` (break `/Game/Systems/Puzzles/FHintPedestalStruct` _returnvalue))))))

(fn `UserConstructionScript`
  (`parent.UserConstructionScript`))