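; Puzzle controller that tracks a set of puzzles and signals when all of them are solved.
; On BeginPlay it binds to the pedestal-updated dispatcher of each entry in Puzzels.
; CheckState exits at the first unsolved entry; otherwise it calls QuitInspection on the loop's last element and fires the OnPuzzleSolved dispatcher.
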(event `self.ReceiveBeginPlay`
  (for _array_element (`self.Puzzels`)
    (add `/Game/Systems/Puzzles/BP_Pedestal.ED_PedestalUpdated` _array_element (`|CreateDelegate` :!event `CheckState`))))

(fn `CheckState`
  (for _array_element (`self.Puzzels`)
    (if (not (`/Game/Systems/Puzzles/BP_Pedestal.IsSolved` _array_element))
      (return)))
  (`/Game/Systems/Masters/BP_MasterStation.QuitInspection` _array_element)
  (`self.OnPuzzleSolved`))

(fn `UserConstructionScript`)