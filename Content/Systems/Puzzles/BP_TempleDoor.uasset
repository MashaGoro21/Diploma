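; Temple door that swings open when its linked puzzle is solved.
; On BeginPlay it binds OpenDoor to the PuzzleController's OnPuzzleSolved dispatcher.
; OpenDoor blends the player's view to the door while a Timeline rotates the Scene component a quarter turn in yaw, then returns the view to the player pawn.
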(event `self.ReceiveBeginPlay`
  (add `/Game/Systems/Puzzles/BP_PuzzleController.OnPuzzleSolved` (`self.PuzzleController`) (delegate `Open Door`)))

(event `Open Door`
  (`PlayerController.SetViewTargetWithBlend` (`GameplayStatics.GetPlayerController` 0) self 0.0 "VTBlend_Linear" 0.0 false)
  (bind (_direction `_новая_дорожка_0`) (`Timeline|Timeline`)
    (:`Update`
      (`SceneComponent.K2_SetRelativeRotation` (`self.Scene`) (`KismetMathLibrary.MakeRotator` 0.0 0.0 (`KismetMathLibrary.Lerp` 0.0 -90.0 `_новая_дорожка_0`)) false false))
    (:`Finished`
      (`PlayerController.SetViewTargetWithBlend` (`GameplayStatics.GetPlayerController` 0) (`GameplayStatics.GetPlayerPawn` 0) 0.0 "VTBlend_Linear" 0.0 false))))

(fn `UserConstructionScript`)