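; BP_SaveGame is a save game object that coordinates saving and loading of data for saveable objects.
; SaveAllData first copies every IsBuildedMapArchive entry into IsBuildedMap, then sends each given object a SaveData interface message with itself as the argument.
; LoadDataForRequester sends a LoadData message back to a single requester, so each object handles its own data against the shared save.
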(fn `IsBuildedMapSave`
  (bind _isbuildedmaparchive (`self.IsBuildedMapArchive`))
  (bind _keys (`BlueprintMapLibrary.Map_Keys` _isbuildedmaparchive))
  (for _array_element _keys
    (`BlueprintMapLibrary.Map_Add` (`self.IsBuildedMap`) _array_element (`.ReturnValue` (`BlueprintMapLibrary.Map_Find` _isbuildedmaparchive _array_element))))
  (return))

(fn `LoadDataForRequester`
  (params (Requester :type "Object Object Reference"))
  (message `/Game/Systems/Save/BPI_Saveable.LoadData` Requester self)
  (return))

(fn `SaveAllData`
  (params (SaveableObjects :type "Array of Object Object Reference"))
  (`self.IsBuildedMapSave`)
  (for _array_element SaveableObjects
    (message `/Game/Systems/Save/BPI_Saveable.SaveData` _array_element self))
  (return))