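; Spawner that fills random zones with copies of a chosen object at BeginPlay, respawning them whenever the first-person player's reset-location dispatcher fires.
; Each run destroys earlier spawns, picks zones (optionally unique per object), then retries random points until one clears the minimum distance from others.
; Spawned objects inherit their zone's rotation and scale and receive the configured physics-simulation setting.
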(event `self.ReceiveBeginPlay`
  (bind _asbp_first_person_character (cast `/Game/FirstPerson/Blueprints/BP_FirstPersonCharacter` (`GameplayStatics.GetPlayerPawn` 0)))
  (set `self.Player` _asbp_first_person_character)
  (add `/Game/FirstPerson/Blueprints/BP_FirstPersonCharacter.ED_ResetLocation` (`self.Player`) (delegate `SpawnObjects`))
  (`self.SpawnObjects`))

(event `SpawnObjects`
  (`self.ClearObjects`)
  (for _ (range (`self.SpawnCount`))
    (bind _zone (`self.GetRandomZone`))
    (`/Engine/EditorBlueprintResources/StandardMacros.IsValid` _zone
      (:`Is Valid`
        (bind _position (`self.FindCorrectLocation` _zone))
        (bind _returnvalue (`self.GetActorScale3D` _zone))
        (bind _returnvalue_2 (`|SpawnActorFromClass` (`self.ObjectToSpawn`) (`KismetMathLibrary.MakeTransform` _position (`self.K2_GetActorRotation` _zone) _returnvalue) "Undefined" "MultiplyWithRoot" null null))
        (`self.SetActorScale3D` _returnvalue_2 _returnvalue)
        (`/Game/Systems/Masters/BP_ObjectMaster.SetPhysicsStatus` _returnvalue_2 (`self.IsSimulatePhysics`))
        (`KismetArrayLibrary.Array_Add` (`self.SpawnedObjects`) _returnvalue_2)))))

(event `ClearObjects`
  (for _array_element (`self.SpawnedObjects`)
    (`/Engine/EditorBlueprintResources/StandardMacros.IsValid` _array_element
      (:`Is Valid`
        (`self.K2_DestroyActor` _array_element))))
  (`KismetArrayLibrary.Array_Clear` (`self.IndicesInUse`))
  (`KismetArrayLibrary.Array_Clear` (`self.SpawnedPositions`))
  (`KismetArrayLibrary.Array_Clear` (`self.SpawnedObjects`)))

(fn `FindCorrectLocation`
  (params (Zone :type "/Game/Systems/Spawner/BP_SpawnZone Object Reference"))
  (returns (Position :type "Vector Structure"))
  (locals (CurrentPosition :type "Vector Structure") (`InSearch?` :type Boolean :default true))
  (bind _currentposition (`local.CurrentPosition`))
  (while (`local.InSearch?`)
    (bind _point (`/Game/Systems/Spawner/BP_SpawnZone.GetRandomPoint` (`local.Zone`)))
    (set `local.CurrentPosition` _point)
    (set `local.InSearch?` false)
    (for _array_element (`self.SpawnedPositions`)
      (bind _output_get (set `local.InSearch?` (< (`KismetMathLibrary.Vector_Distance` _array_element (`local.CurrentPosition`)) (`self.MinDistance`))))
      (if _output_get
        (break))))
  (`KismetArrayLibrary.Array_Add` (`self.SpawnedPositions`) _currentposition)
  (return _currentposition))

(fn `GetRandomZone`
  (returns (Zone :type "/Game/Systems/Spawner/BP_SpawnZone Object Reference"))
  (locals (CurrentIndex :type Integer) (`Found?` :type Boolean))
  (bind _currentindex (`local.CurrentIndex`))
  (if (`self.OnePerOne`)
    (if (> (`self.SpawnCount`) (`KismetArrayLibrary.Array_Length` (`self.SpawnZones`)))
      (`KismetSystemLibrary.PrintString` "Spawn Count Greater Zones Lenght!")
      (else
        (while (not (`local.Found?`))
          (bind _output_get (set `local.CurrentIndex` (`.OutIndex` (`KismetArrayLibrary.Array_Random` (`self.SpawnZones`)))))
          (set `local.Found?` (== (`KismetArrayLibrary.Array_Find` (`self.IndicesInUse`) _output_get) -1)))
        (`KismetArrayLibrary.Array_Add` (`self.IndicesInUse`) _currentindex)
        (return (`|GetArrayItem` (`self.SpawnZones`) _currentindex))))
    (else
      (return (`KismetArrayLibrary.Array_Random` (`self.SpawnZones`))))))

(fn `UserConstructionScript`)