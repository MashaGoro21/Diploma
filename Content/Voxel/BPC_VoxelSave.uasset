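; Blueprint component that saves and restores the VoxelWorld terrain through the game's save system.
; On BeginPlay it binds to the voxel world's load event, then either stores an async compressed snapshot for a new game or requests a load from the game instance.
; SaveData and LoadData handlers write and apply the compressed voxel save held in the SaveGame object.
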(event `self.ReceiveBeginPlay`
  (bind _returnvalue (`GameplayStatics.GetActorOfClass` "/Script/Voxel.VoxelWorld"))
  (bind _output_get (set `self.VoxelWorld` _returnvalue))
  (bind _asbp_game_instance (cast `/Game/Systems/Save/BP_GameInstance` (`GameplayStatics.GetGameInstance`)))
  (add `VoxelWorld.OnWorldLoaded` _output_get (delegate `VoxelSave/Load`)))

(event `VoxelSave/Load`
  (if (`/Game/Systems/Save/BP_GameInstance.IsNewGame` (stale `self.ReceiveBeginPlay` _asbp_game_instance))
    (bind _outsave (`VoxelDataTools.GetCompressedSaveAsync` (`self.VoxelWorld`)))
    (set `/Game/Systems/Save/BP_SaveGame.VoxelWorld` _outsave (`/Game/Systems/Save/BP_GameInstance.SaveGameRef` (stale `self.ReceiveBeginPlay` _asbp_game_instance)))
    (else
      (message `/Game/Systems/Save/BPI_Persistence.RequestLoad` (`GameplayStatics.GetGameInstance`) self))))

(event `/Game/Systems/Save/BPI_Saveable.LoadData`
  (params (SaveGameRef :type "/Game/Systems/Save/BP_SaveGame Object Reference"))
  (bind _returnvalue (`GameplayStatics.GetActorOfClass` "/Script/Voxel.VoxelWorld"))
  (`VoxelDataTools.LoadFromCompressedSave` _returnvalue (`/Game/Systems/Save/BP_SaveGame.VoxelWorld` SaveGameRef)))

(event `/Game/Systems/Save/BPI_Saveable.SaveData`
  (params (SaveGameRef :type "/Game/Systems/Save/BP_SaveGame Object Reference"))
  (bind _returnvalue (`GameplayStatics.GetActorOfClass` "/Script/Voxel.VoxelWorld"))
  (bind _outsave (`VoxelDataTools.GetCompressedSave` _returnvalue))
  (set `/Game/Systems/Save/BP_SaveGame.VoxelWorld` _outsave SaveGameRef))